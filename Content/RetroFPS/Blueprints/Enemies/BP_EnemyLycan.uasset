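; Lycan enemy for a retro FPS, a flipbook-sprite pawn that chases the player and deals contact damage on capsule overlap.
; Tick turns it toward a seen player, or picks front or back idle sprites by dot-product angle until then.
; Sight or non-lethal damage starts the AIMoveTo chase, while hits play a flinch and lethal damage plays death before destroying it.
; An eight-direction view using Helldog sprites is left unused.
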(event `self.ReceiveTick`
  (params (DeltaSeconds :type "Float (single-precision)"))
  (bind (_returnvalue_roll _returnvalue_pitch _returnvalue_yaw) (`KismetMathLibrary.BreakRotator` (`KismetMathLibrary.FindLookAtRotation` (`self.K2_GetActorLocation`) (`self.K2_GetActorLocation` (`GameplayStatics.GetPlayerCharacter` 0)))))
  (bind _returnvalue (`KismetMathLibrary.Normal` (- (`self.K2_GetActorLocation` (`GameplayStatics.GetPlayerCharacter` 0)) (`self.K2_GetActorLocation`))))
  ;[0 0 0] Rotate to Player
  (if (`self.CanSeePlayer`)
    (`self.K2_SetActorRotation` (`KismetMathLibrary.MakeRotator` 0.0 0.0 _returnvalue_yaw))
    (if (`self.Dead`)
      _
      (elif (not (`self.Flinch`))
        (`PaperFlipbookComponent.SetFlipbook` (`self.PaperFlipbook`) "/Game/RetroFPS/Flipbooks/Werewolf/FB_LycanWalk.FB_LycanWalk")))
    (elif (`self.Flinch`)
      _
      (elif (not (`self.Dead`))
        (set `self.Degrees` (`KismetMathLibrary.DegAcos` (`KismetMathLibrary.Dot_VectorVector` (`self.GetActorForwardVector`) _returnvalue)))
        (if (< (`KismetMathLibrary.Dot_VectorVector` (`self.GetActorRightVector`) _returnvalue) 0.0)
          (`/Engine/EditorBlueprintResources/StandardMacros.CompareFloat` (`self.Degrees`) 90.0 ; Left Side
            (:`>`
              (`SceneComponent.K2_SetRelativeRotation` (`self.PaperFlipbook`) (struct :`Yaw` 90.0) false false :!label _label)
              (`PaperFlipbookComponent.SetFlipbook` (`self.PaperFlipbook`) "/Game/RetroFPS/Flipbooks/Werewolf/FB_LycanIdleBack.FB_LycanIdleBack"))
            (:`==`
              (goto _label))
            (:`<`
              (`SceneComponent.K2_SetRelativeRotation` (`self.PaperFlipbook`) (struct :`Yaw` 90.0) false false)
              (`PaperFlipbookComponent.SetFlipbook` (`self.PaperFlipbook`) "/Game/RetroFPS/Flipbooks/Werewolf/FB_LycanIdle.FB_LycanIdle")))
          (else
            (`/Engine/EditorBlueprintResources/StandardMacros.CompareFloat` (`self.Degrees`) 90.0 ; Right Side
              (:`>`
                (`SceneComponent.K2_SetRelativeRotation` (`self.PaperFlipbook`) (struct :`Yaw` 90.0) false false :!label _label_2)
                (`PaperFlipbookComponent.SetFlipbook` (`self.PaperFlipbook`) "/Game/RetroFPS/Flipbooks/Werewolf/FB_LycanIdleBack.FB_LycanIdleBack"))
              (:`==`
                (goto _label_2))
              (:`<`
                (`SceneComponent.K2_SetRelativeRotation` (`self.PaperFlipbook`) (struct :`Yaw` 90.0) false false)
                (`PaperFlipbookComponent.SetFlipbook` (`self.PaperFlipbook`) "/Game/RetroFPS/Flipbooks/Werewolf/FB_LycanIdle.FB_LycanIdle")))))))))

(event `self.PawnSensing.OnSeePawn`
  (params (Pawn :type "Pawn Object Reference"))
  ;[0 0 0] See Player
  (bind _asbp_fpsplayer (cast `/Game/RetroFPS/Blueprints/BP_FPSPlayer` Pawn))
  (set `self.CanSeePlayer` true)
  (`|AIMoveTo` self (0.0 0.0 0.0) _asbp_fpsplayer
    (:`then`
      (`/Engine/EditorBlueprintResources/StandardMacros.DoOnce` false
        (:`Completed`
          (`GameplayStatics.PlaySound2D` "/Game/RetroFPS/Sound/Helldog/HelldogAggroCUE.HelldogAggroCUE" 1.0 1.0 0.0 null null))))))

(event `self.ReceiveAnyDamage`
  (params (Damage :type "Float (single-precision)") (DamageType :type "DamageType Object Reference") (InstigatedBy :type "Controller Object Reference") (DamageCauser :type "Actor Object Reference"))
  (bind _paperflipbook (`self.PaperFlipbook`))
  (bind _paperflipbook_2 (`self.PaperFlipbook`))
  (bind (_returnvalue_roll _returnvalue_pitch _returnvalue_yaw) (`KismetMathLibrary.BreakRotator` (`KismetMathLibrary.FindLookAtRotation` (`self.K2_GetActorLocation`) (`self.K2_GetActorLocation` (`GameplayStatics.GetPlayerCharacter` 0)))))
  ;[0 0 0] Death Animation & Take Damage
  (set `self.Health` (- (`self.Health`) Damage))
  (if (>= (`self.Health`) 1.0)
    (`GameplayStatics.PlaySound2D` "/Game/RetroFPS/Sound/Lycan/LycanHurt.LycanHurt" 1.0 1.0 0.0 null null)
    (`ActorComponent.Deactivate` (`self.CharacterMovement`))
    (set `self.Flinch` true)
    (`PaperFlipbookComponent.SetFlipbook` _paperflipbook "/Game/RetroFPS/Flipbooks/Werewolf/FB_LycanDamage.FB_LycanDamage")
    (`KismetSystemLibrary.Delay` (`PaperFlipbookComponent.GetFlipbookLength` _paperflipbook))
    (set `self.Flinch` false)
    (`self.K2_SetActorRotation` (`KismetMathLibrary.MakeRotator` 0.0 0.0 _returnvalue_yaw))
    (`ActorComponent.Activate` (`self.CharacterMovement`) false)
    (`PaperFlipbookComponent.SetFlipbook` (`self.PaperFlipbook`) "/Game/RetroFPS/Flipbooks/Werewolf/FB_LycanIdle.FB_LycanIdle")
    (set `self.CanSeePlayer` true)
    (`|AIMoveTo` self (0.0 0.0 0.0) (`GameplayStatics.GetPlayerCharacter` 0)
      (:`then`
        (`/Engine/EditorBlueprintResources/StandardMacros.DoOnce` false
          (:`Completed`
            (`GameplayStatics.PlaySound2D` "/Game/RetroFPS/Sound/Helldog/HelldogAggroCUE.HelldogAggroCUE" 1.0 1.0 0.0 null null)))))
    (else
      (`GameplayStatics.PlaySound2D` "/Game/RetroFPS/Sound/Lycan/LycanDeath.LycanDeath" 1.0 1.0 0.0 null null)
      (`ActorComponent.Deactivate` (`self.CharacterMovement`))
      (set `self.Flinch` true)
      (`PaperFlipbookComponent.SetFlipbook` _paperflipbook_2 "/Game/RetroFPS/Flipbooks/Werewolf/FB_LycanDeath.FB_LycanDeath")
      (`KismetSystemLibrary.Delay` (`PaperFlipbookComponent.GetFlipbookLength` _paperflipbook_2))
      (set `self.Flinch` false)
      (set `self.Dead` true)
      (`PaperFlipbookComponent.SetFlipbook` (`self.PaperFlipbook`) "/Game/RetroFPS/Flipbooks/Werewolf/FB_LycanDead.FB_LycanDead")
      (`ActorComponent.SetActive` (`self.CapsuleComponent`) false false)
      (`KismetSystemLibrary.Delay` 4.0)
      (`self.K2_DestroyActor`))))

(event `self.CapsuleComponent.OnComponentBeginOverlap`
  (params (OverlappedComponent :type "PrimitiveComponent Object Reference") (OtherActor :type "Actor Object Reference") (OtherComp :type "PrimitiveComponent Object Reference") (OtherBodyIndex :type Integer) (bFromSweep :type Boolean) (SweepResult :type "HitResult Structure (by ref)"))
  (if (not (`self.Dead`))
    (bind _asbp_fpsplayer (cast `/Game/RetroFPS/Blueprints/BP_FPSPlayer` OtherActor))
    (`GameplayStatics.ApplyDamage` _asbp_fpsplayer 45.0 null self)))

(fn `UserConstructionScript`)