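; BP_FPSPlayer is the retro FPS player character, handling movement, mouse look, shooting, damage and healing.
; It spawns weapons through a child actor component, initializes them via I_PlayerWeapon and drives their bobbing from movement each Tick.
; It pushes health and ammo to WBP_HUD and only fires while ammo remains.
; Death destroys the actor, and its Destroyed event asks BP_FPSGameMode to respawn it, with the transform saved at BeginPlay.
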(event `self.ReceiveBeginPlay`
  ;[0 0 0] Begin Play
  (`|ExecutionSequence`
    (:`then_0`
      (bind _returnvalue (`|CreateWidget` "/Game/RetroFPS/Blueprints/WBP_HUD.WBP_HUD_C"))
      (bind _output_get (set `self.HUDRef` _returnvalue))
      (`UserWidget.AddToViewport` _output_get 0)
      (`self.Equip Weapon` "/Game/RetroFPS/Blueprints/BP_PlayerWeaponBase.BP_PlayerWeaponBase_C")
      (bind _asbp_fpsgame_mode (cast `/Game/RetroFPS/Blueprints/BP_FPSGameMode` (`GameplayStatics.GetGameMode`)))
      (set `/Game/RetroFPS/Blueprints/BP_FPSGameMode.Respawn Transform` (`self.GetTransform`) _asbp_fpsgame_mode))))

(event `InputAxis|HorizontalMovement`
  (params (AxisValue :type "Float (single-precision)"))
  (bind (_returnvalue_roll _returnvalue_pitch _returnvalue_yaw) (`KismetMathLibrary.BreakRotator` (`self.GetControlRotation`)))
  ;[0 0 0] Main Movement
  (`self.AddMovementInput` (`KismetMathLibrary.GetRightVector` (`KismetMathLibrary.MakeRotator` 0.0 0.0 _returnvalue_yaw)) AxisValue))

(event `InputAxis|VerticalMovement`
  (params (AxisValue :type "Float (single-precision)"))
  (bind (_returnvalue_roll _returnvalue_pitch _returnvalue_yaw) (`KismetMathLibrary.BreakRotator` (`self.GetControlRotation`)))
  ;[0 0 0] Main Movement
  (`self.AddMovementInput` (`KismetMathLibrary.GetForwardVector` (`KismetMathLibrary.MakeRotator` 0.0 0.0 _returnvalue_yaw)) AxisValue))

(event `InputAxis|MouseLookHorizontal`
  (params (AxisValue :type "Float (single-precision)"))
  ;[0 0 0] Mouse Look
  (`self.AddControllerYawInput` AxisValue))

(event `self.ReceiveTick`
  (params (DeltaSeconds :type "Float (single-precision)"))
  ;[0 0 0] WeaponBob
  (bind _asbp_player_weapon_base (cast `/Game/RetroFPS/Blueprints/BP_PlayerWeaponBase` (`ChildActorComponent.ChildActor` (`self.Weapon`))))
  (`/Game/RetroFPS/Blueprints/BP_PlayerWeaponBase.Weapon Bobbing` _asbp_player_weapon_base (> (`KismetMathLibrary.VSize` (`MovementComponent.Velocity` (`self.CharacterMovement`))) 0.0) DeltaSeconds)
  (set `/Game/RetroFPS/Blueprints/WBP_HUD.Ammo` (`self.Ammo`) (`self.HUDRef`)))

(event `InputAxis|MouseLookVertical`
  (params (AxisValue :type "Float (single-precision)"))
  ;[0 0 0] Mouse Look
  (`self.AddControllerPitchInput` AxisValue))

(event `Equip Weapon`
  (params (Weapon :type "/Game/RetroFPS/Blueprints/BP_PlayerWeaponBase Class Reference"))
  (bind _weapon (`self.Weapon`))
  (bind _childactor (`ChildActorComponent.ChildActor` _weapon))
  ;[0 0 0] Equip Weapon
  (bind _output_get (set `self.Current Weapon Class` Weapon))
  (`ChildActorComponent.SetChildActorClass` _weapon _output_get)
  (if (`KismetSystemLibrary.DoesImplementInterface` _childactor "/Game/RetroFPS/Blueprints/I_PlayerWeapon.I_PlayerWeapon_C")
    (message `/Game/RetroFPS/Blueprints/I_PlayerWeapon.InitializeWeapon` _childactor)
    (bind _asbp_player_weapon_base (cast `/Game/RetroFPS/Blueprints/BP_PlayerWeaponBase` _childactor))
    (bind _output_get_2 (set `self.Current Weapon` _asbp_player_weapon_base))
    (`MovieSceneSequencePlayer.Play` (`ActorSequenceComponent.SequencePlayer` (`/Game/RetroFPS/Blueprints/BP_PlayerWeaponBase.Weapon Draw` _output_get_2)))
    (`KismetSystemLibrary.Delay` 0.2)
    (set `/Game/RetroFPS/Blueprints/WBP_HUD.Ammo` (`self.Ammo`) (`self.HUDRef`))))

(event `InputAction|Shoot`
  (params (Key :type "Key Structure"))
  ;[0 0 0] Shoot
  (:`Pressed`
    (if (> (`self.Ammo`) 0)
      (`/Game/RetroFPS/Blueprints/BP_PlayerWeaponBase.Shoot` (`self.Current Weapon`))
      (elif (`self.GunEquipped`)
        (`GameplayStatics.PlaySound2D` "/Game/RetroFPS/Sound/Player/ClipEmpty.ClipEmpty" 1.0 1.0 0.0 null null)))))

(event `self.ReceiveAnyDamage`
  (params (Damage :type "Float (single-precision)") (DamageType :type "DamageType Object Reference") (InstigatedBy :type "Controller Object Reference") (DamageCauser :type "Actor Object Reference"))
  ;[0 0 0] Take Damage & Death
  (if (not (`self.IsDead`))
    (bind _output_get (set `self.Health` (`KismetMathLibrary.FClamp` (- (`self.Health`) Damage) 0.0 (`self.MaxHealth`))))
    (bind _output_get_2 (set `/Game/RetroFPS/Blueprints/WBP_HUD.Health` _output_get (`self.HUDRef`)))
    (if (== _output_get_2 0.0)
      (`GameplayStatics.PlaySound2D` "/Game/RetroFPS/Sound/Player/PlayerDeath.PlayerDeath" 1.0 1.0 0.0 null null)
      (set `self.IsDead` true)
      (`ActorComponent.Deactivate` (`self.CharacterMovement`))
      (`KismetSystemLibrary.Delay` 1.0)
      (`self.K2_DestroyActor`)
      (else
        (`GameplayStatics.PlaySound2D` "/Game/RetroFPS/Sound/Player/PlayerHurtCUE.PlayerHurtCUE" 1.0 1.0 0.0 null null)))))

(event `Heal Player`
  (params (`Heal Value` :type "Float (double-precision)"))
  ;[0 0 0] Healing System
  (if (and (not (`self.IsDead`)) (!= (`self.Health`) (`self.MaxHealth`)))
    (bind _output_get (set `self.Health` (`KismetMathLibrary.FClamp` (+ `Heal Value` (`self.Health`)) 0.0 (`self.MaxHealth`))))
    (set `/Game/RetroFPS/Blueprints/WBP_HUD.Health` _output_get (`self.HUDRef`))
    (`GameplayStatics.PlaySound2D` "/Game/RetroFPS/Sound/Player/PlayerHealing.PlayerHealing" 1.0 1.0 0.0 null null)))

(event `self.ReceiveDestroyed`
  ;[0 0 0] Death
  (bind _asbp_fpsgame_mode (cast `/Game/RetroFPS/Blueprints/BP_FPSGameMode` (`GameplayStatics.GetGameMode`)))
  (`/Game/RetroFPS/Blueprints/BP_FPSGameMode.RespawnPlayer` _asbp_fpsgame_mode self))

(fn `UserConstructionScript`)