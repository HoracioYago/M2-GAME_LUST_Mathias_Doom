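; Ammo pickup for the retro FPS that refills the player's ammo to its maximum on contact.
; Overlap with BP_FPSPlayer only takes effect if a gun is equipped, then plays a reload sound and destroys the pickup.
; Each Tick, the AmmoPack component turns on yaw alone to face the player camera, with a 90-degree offset, acting as an upright billboard.
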(event `self.ReceiveActorBeginOverlap`
  (params (OtherActor :type "Actor Object Reference"))
  ;[0 0 0] Pick Up / Player Contact
  (bind _asbp_fpsplayer (cast `/Game/RetroFPS/Blueprints/BP_FPSPlayer` OtherActor))
  (if (`/Game/RetroFPS/Blueprints/BP_FPSPlayer.GunEquipped` _asbp_fpsplayer)
    (`GameplayStatics.PlaySound2D` "/Game/RetroFPS/Sound/Player/Reload.Reload" 1.0 1.0 0.0 null null)
    (set `/Game/RetroFPS/Blueprints/BP_FPSPlayer.Ammo` (`/Game/RetroFPS/Blueprints/BP_FPSPlayer.AmmoMax` _asbp_fpsplayer) _asbp_fpsplayer)
    (`self.K2_DestroyActor`)))

(event `self.ReceiveTick`
  (params (DeltaSeconds :type "Float (single-precision)"))
  (bind _ammopack (`self.AmmoPack`))
  (bind (_returnvalue_roll _returnvalue_pitch _returnvalue_yaw) (`KismetMathLibrary.BreakRotator` (`KismetMathLibrary.FindLookAtRotation` (`SceneComponent.K2_GetComponentLocation` _ammopack) (`PlayerCameraManager.GetCameraLocation` (`GameplayStatics.GetPlayerCameraManager` 0)))))
  ;[0 0 0] Constant Rotation
  (`SceneComponent.K2_SetWorldRotation` _ammopack (`KismetMathLibrary.MakeRotator` 0.0 0.0 (- _returnvalue_yaw 90.0)) false false))

(fn `UserConstructionScript`)