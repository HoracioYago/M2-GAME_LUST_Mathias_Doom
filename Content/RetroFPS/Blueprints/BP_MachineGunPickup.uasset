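; BP_MachineGunPickup is a weapon pickup that equips the player with a weapon on contact.
; On overlap with BP_FPSPlayer it equips WeaponToAcquire, fills ammo, flags the gun as equipped, sets damage on WeaponBase, then destroys itself.
; Each tick it yaws the Weapon component toward the player camera with a 90-degree offset, billboard-style, keeping pitch and roll at zero.
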(event `self.ReceiveActorBeginOverlap`
  (params (OtherActor :type "Actor Object Reference"))
  ;[0 0 0] Pick Up / Player Contact
  (bind _asbp_fpsplayer (cast `/Game/RetroFPS/Blueprints/BP_FPSPlayer` OtherActor))
  (`/Game/RetroFPS/Blueprints/BP_FPSPlayer.Equip Weapon` _asbp_fpsplayer (`self.Weapon to Acquire`))
  (set `/Game/RetroFPS/Blueprints/BP_FPSPlayer.AmmoMax` 30 _asbp_fpsplayer)
  (set `/Game/RetroFPS/Blueprints/BP_FPSPlayer.Ammo` 30 _asbp_fpsplayer)
  (set `/Game/RetroFPS/Blueprints/BP_FPSPlayer.GunEquipped` true _asbp_fpsplayer)
  (set `/Game/RetroFPS/Blueprints/BP_PlayerWeaponBase.WeaponDamage` 3.0 (`self.Weapon Base`))
  (`self.K2_DestroyActor`))

(event `self.ReceiveTick`
  (params (DeltaSeconds :type "Float (single-precision)"))
  (bind _weapon (`self.Weapon`))
  (bind (_returnvalue_roll _returnvalue_pitch _returnvalue_yaw) (`KismetMathLibrary.BreakRotator` (`KismetMathLibrary.FindLookAtRotation` (`SceneComponent.K2_GetComponentLocation` _weapon) (`PlayerCameraManager.GetCameraLocation` (`GameplayStatics.GetPlayerCameraManager` 0)))))
  ;[0 0 0] Constant Rotation
  (`SceneComponent.K2_SetWorldRotation` _weapon (`KismetMathLibrary.MakeRotator` 0.0 0.0 (- _returnvalue_yaw 90.0)) false false))

(fn `UserConstructionScript`)