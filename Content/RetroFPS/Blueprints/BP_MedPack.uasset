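; BP_MedPack is a health pickup for the RetroFPS game.
; When a BP_FPSPlayer below max health overlaps it, it calls HealPlayer with that player's MaxHealth and destroys itself, so a player at full health leaves it in place.
; Every tick it yaws the MedPack component toward the player camera with a 90-degree offset and zero pitch and roll, acting as a vertical-axis billboard.
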(event `self.ReceiveActorBeginOverlap`
  (params (OtherActor :type "Actor Object Reference"))
  ;[0 0 0] Pick Up / Player Contact
  (bind _asbp_fpsplayer (cast `/Game/RetroFPS/Blueprints/BP_FPSPlayer` OtherActor))
  (if (< (`/Game/RetroFPS/Blueprints/BP_FPSPlayer.Health` _asbp_fpsplayer) (`/Game/RetroFPS/Blueprints/BP_FPSPlayer.MaxHealth` _asbp_fpsplayer))
    (`/Game/RetroFPS/Blueprints/BP_FPSPlayer.Heal Player` _asbp_fpsplayer (`/Game/RetroFPS/Blueprints/BP_FPSPlayer.MaxHealth` _asbp_fpsplayer))
    (`self.K2_DestroyActor`)))

(event `self.ReceiveTick`
  (params (DeltaSeconds :type "Float (single-precision)"))
  (bind _medpack (`self.MedPack`))
  (bind (_returnvalue_roll _returnvalue_pitch _returnvalue_yaw) (`KismetMathLibrary.BreakRotator` (`KismetMathLibrary.FindLookAtRotation` (`SceneComponent.K2_GetComponentLocation` _medpack) (`PlayerCameraManager.GetCameraLocation` (`GameplayStatics.GetPlayerCameraManager` 0)))))
  ;[0 0 0] Constant Rotation
  (`SceneComponent.K2_SetWorldRotation` _medpack (`KismetMathLibrary.MakeRotator` 0.0 0.0 (- _returnvalue_yaw 90.0)) false false))

(fn `UserConstructionScript`)