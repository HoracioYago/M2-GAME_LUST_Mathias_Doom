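; BP_MachineGun is a retro FPS weapon that fires a three-shot burst with flipbook sprite animation.
; Shoot passes a DoOnce gate, calls FireWeapon three times at once, then shows the shot flipbook and muzzle light and plays a sound.
; After a delay of one flipbook length, it restores the idle look, deducts three ammo from BP_FPSPlayer and resets the gate.
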(event `self.InitializeWeapon`
  ;[0 0 0] Initialize Weapon
  (`PaperFlipbookComponent.SetFlipbook` (`self.Weapon Flipbook`) (`self.Idle Rifle`))
  (`SceneComponent.SetHiddenInGame` (`self.Weapon Flipbook`) false false))

(event `self.Shoot`
  (bind _weapon_flipbook (`self.Weapon Flipbook`))
  ;[0 0 0] Shoot Logic & Switch Flipbook
  (`/Engine/EditorBlueprintResources/StandardMacros.DoOnce` false :!label _label
    (:`Completed`
      (`self.FireWeapon`)
      (`self.FireWeapon`)
      (`self.FireWeapon`)
      (`PaperFlipbookComponent.SetFlipbook` _weapon_flipbook "/Game/RetroFPS/Flipbooks/FB_RifleShot.FB_RifleShot")
      (`SceneComponent.SetHiddenInGame` (`self.PointLight`) false false)
      (`GameplayStatics.PlaySound2D` "/Game/RetroFPS/Sound/Player/MachineGun.MachineGun" 1.0 1.0 0.0 null null)
      (`KismetSystemLibrary.Delay` (`PaperFlipbookComponent.GetFlipbookLength` _weapon_flipbook))
      (`SceneComponent.SetHiddenInGame` (`self.PointLight`) true false)
      (`PaperFlipbookComponent.SetFlipbook` (`self.Weapon Flipbook`) "/Game/RetroFPS/Flipbooks/FB_RifleIdle.FB_RifleIdle")
      (bind _asbp_fpsplayer (cast `/Game/RetroFPS/Blueprints/BP_FPSPlayer` (`GameplayStatics.GetPlayerCharacter` 0)))
      (set `/Game/RetroFPS/Blueprints/BP_FPSPlayer.Ammo` (- (`/Game/RetroFPS/Blueprints/BP_FPSPlayer.Ammo` _asbp_fpsplayer) 3) _asbp_fpsplayer)
      (`self.Reset Weapon`))))

(event `Reset Weapon`
  ;[0 0 0] Shoot Logic & Switch Flipbook
  (goto _label :!via `Reset`))

(fn `UserConstructionScript`
  (`parent.UserConstructionScript`))