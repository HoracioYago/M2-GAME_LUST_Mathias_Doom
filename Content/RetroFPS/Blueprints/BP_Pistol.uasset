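; Pistol weapon Blueprint for a retro FPS, using Paper2D flipbooks for its idle and firing visuals.
; InitializeWeapon sets the idle flipbook and makes it visible.
; Shoot passes a DoOnce gate, calls FireWeapon, plays the fire flipbook for its length, then restores idle and resets the gate.
; The gate blocks repeat shots until the animation delay ends or ResetWeapon is called.
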(event `/Game/RetroFPS/Blueprints/I_PlayerWeapon.InitializeWeapon`
  ;[0 0 0] Initialize Weapon
  (`PaperFlipbookComponent.SetFlipbook` (`self.Weapon Flipbook`) (`self.Idle Pistol`))
  (`SceneComponent.SetHiddenInGame` (`self.Weapon Flipbook`) false false))

(event `self.Shoot`
  (bind _weapon_flipbook (`self.Weapon Flipbook`))
  ;[0 0 0] Shoot Logic & Switch Flipbook
  (`/Engine/EditorBlueprintResources/StandardMacros.DoOnce` false :!label _label
    (:`Completed`
      (`self.FireWeapon`)
      (`PaperFlipbookComponent.SetFlipbook` _weapon_flipbook "/Game/RetroFPS/Flipbooks/FB_PistolFire.FB_PistolFire")
      (`KismetSystemLibrary.Delay` (`PaperFlipbookComponent.GetFlipbookLength` _weapon_flipbook))
      (`PaperFlipbookComponent.SetFlipbook` (`self.Weapon Flipbook`) "/Game/RetroFPS/Flipbooks/FB_PistolIdle.FB_PistolIdle")
      (`self.Reset Weapon`))))

(event `Reset Weapon`
  ;[0 0 0] Shoot Logic & Switch Flipbook
  (goto _label :!via `Reset`))

(fn `UserConstructionScript`
  (`parent.UserConstructionScript`))